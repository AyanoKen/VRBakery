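; BP_ColorChanging is a physics prop that takes the shape of a random bed part and can switch to a random material.
; Its construction script draws a mesh from BedParts in BP_GameInstance, enables physics with a raised mass scale, then removes that mesh from the shared list so later instances draw others.
; The ChangeColor event applies a random entry from Materials to the mesh's first material slot.
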(event Custom|ChangeColor
  (Rendering|Material|SetMaterial (Variables|Default|GetStaticMesh) 0 (.OutItem (Utilities|Array|Random (Variables|Default|GetMaterials)))))

(event EventBeginPlay
  (|CallParentFunction) ; This node is disabled and will not be called.\nDrag off pins to build functionality.
)

(event Collision|EventActorBeginOverlap
  (params (OtherActor :type Actor%20Object%20Reference))
  (|CallParentFunction OtherActor) ; This node is disabled and will not be called.\nDrag off pins to build functionality.
)

(event EventTick
  (params (DeltaSeconds :type Float%20%28single-precision%29))
  (|CallParentFunction DeltaSeconds) ; This node is disabled and will not be called.\nDrag off pins to build functionality.
)

(fn ConstructionScript
  (bind _staticmesh (Variables|Default|GetStaticMesh))
  (bind _asbp_game_instance (Utilities|Casting|CastToBP_GameInstance (Game|GetGameInstance)))
  (Components|StaticMesh|SetStaticMesh _staticmesh (.OutItem (Utilities|Array|Random (Variables|/Game/MyGame/Blueprints/BP_GameInstance.BP_GameInstance_C|GetBedParts _asbp_game_instance))))
  (Physics|SetSimulatePhysics _staticmesh true)
  (Class|PrimitiveComponent|SetMassScale _staticmesh "None" 2.0)
  (Utilities|Array|RemoveItem (Variables|/Game/MyGame/Blueprints/BP_GameInstance.BP_GameInstance_C|GetBedParts _asbp_game_instance) (Variables|/Script/Engine.StaticMeshComponent|GetStaticMesh (Variables|Default|GetStaticMesh))))